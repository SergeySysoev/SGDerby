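; BP_Derby_GM is the derby game mode Blueprint that ends the match once no enemies are left.
; BeginPlay caches BP_Derby_GI and resets its EnemiesLeft counter to a hardcoded starting count.
; Tick polls that counter and, once at zero, destroys the player pawn and calls EndGame on BP_Derby_PC.
; The K key handler loops over enemy vehicles with an empty body, and pause-menu logic is left unconnected.
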(event EventBeginPlay
  (bind _asbp_derby_gi (Utilities|Casting|CastToBP_Derby_GI (Game|GetGameInstance)))
  (bind _output_get (Variables|Default|SetAs%20BP%20Derby%20GI _asbp_derby_gi))
  (Variables|/Game/-Derby/Blueprints/Core/BP_Derby_GI.BP_Derby_GI_C|SetEnemiesLeft _output_get 6))

(event EventTick
  (params (DeltaSeconds :type Float%20%28single-precision%29))
  (bind _returnvalue (Game|Player|GetPlayerPawn 0))
  (if (== (Variables|/Game/-Derby/Blueprints/Core/BP_Derby_GI.BP_Derby_GI_C|GetEnemiesLeft (Variables|Default|GetAs%20BP%20Derby%20GI)) 0)
    (Utilities|FlowControl|DoOnce false
      (:Completed
        (if (Utilities|IsValid _returnvalue)
          (Actor|DestroyActor _returnvalue))
        (Default|EndGame (.AsBP%20Derby%20PC (Utilities|Casting|CastToBP_Derby_PC (Game|GetPlayerController 0))))))))

(event Input|KeyboardEvents|K
  (params (Key :type Key%20Structure :default "None"))
  (:Pressed
    (bind _outactors (Actor|GetAllActorsOfClass "/Game/-Derby/Blueprints/Car/BP_AI_Vehicle_Enemy.BP_AI_Vehicle_Enemy_C"))
    (for _array_element _outactors
      _)))

(fn ConstructionScript)