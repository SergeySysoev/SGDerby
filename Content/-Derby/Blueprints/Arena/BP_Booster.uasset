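; BP_Booster is an arena shield pickup that shields the vehicle driving into it.
; It activates its SpawnParticle effect on BeginPlay and waits for an overlap on its Collision component.
; The overlapping actor's display name is checked for "Enemy" or "Ally" to pick the AI vehicle cast, falling back to the player vehicle.
; A successful cast sets that vehicle's IsShielded flag and destroys the booster.
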(event OnComponentBeginOverlap(Collision)
  (params (OverlappedComponent :type Primitive%20Component%20Object%20Reference) (OtherActor :type Actor%20Object%20Reference) (OtherComp :type Primitive%20Component%20Object%20Reference) (OtherBodyIndex :type Integer) (bFromSweep :type Boolean) (SweepResult :type Hit%20Result%20Structure%20%28by%20ref%29))
  (bind _returnvalue (Utilities|GetDisplayName OtherActor))
  (if (Utilities|IsValid OtherActor)
    (if (Utilities|String|Contains _returnvalue "Enemy")
      (bind _asbp_ai_vehicle_enemy (Utilities|Casting|CastToBP_AI_Vehicle_Enemy OtherActor))
      (Variables|/Game/-Derby/Blueprints/Car/BP_AI_Vehicle_Enemy.BP_AI_Vehicle_Enemy_C|SetisShielded _asbp_ai_vehicle_enemy true)
      (Actor|DestroyActor)
      (elif (Utilities|String|Contains _returnvalue "Ally")
        (bind _asbp_ai_vehicle_ally (Utilities|Casting|CastToBP_AI_Vehicle_Ally OtherActor))
        (Variables|/Game/-Derby/Blueprints/Car/BP_AI_Vehicle_Ally.BP_AI_Vehicle_Ally_C|SetisShielded _asbp_ai_vehicle_ally true)
        (Actor|DestroyActor)
        (else
          (bind _asbp_player_vehicle (Utilities|Casting|CastToBP_Player_Vehicle OtherActor))
          (Variables|/Game/-Derby/Blueprints/Car/BP_Player_Vehicle.BP_Player_Vehicle_C|SetisShielded _asbp_player_vehicle true)
          (Actor|DestroyActor))))))

(event EventBeginPlay
  (Components|Activation|Activate (Variables|Default|GetSpawn_Particle) true))

(event Collision|EventActorBeginOverlap
  (params (OtherActor :type Actor%20Object%20Reference)))

(event EventTick
  (params (DeltaSeconds :type Float%20%28single-precision%29)))

(fn ConstructionScript)